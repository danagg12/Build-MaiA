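; BP_PlataformaMovil is a moving platform that shuttles back and forth along the world X axis in an endless loop.
; From BeginPlay, latent MoveComponentTo calls move DefaultSceneRoot out and back by a fixed offset from the current actor location, pausing briefly after each leg.
; The custom event Resetmovimiento calls itself after the return leg to repeat the cycle, without Tick or a Timeline.
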(event `Reset movimiento`
  (`KismetSystemLibrary.MoveComponentTo` (`self.DefaultSceneRoot`) (+ (`self.K2_GetActorLocation`) (600.0 0.0 0.0)) (struct) false false 2.0 :!label _label)
  (`KismetSystemLibrary.Delay` 0.5)
  (`KismetSystemLibrary.MoveComponentTo` (`self.DefaultSceneRoot`) (+ (`self.K2_GetActorLocation`) (-600.0 0.0 0.0)) (struct) false false 2.0)
  (`KismetSystemLibrary.Delay` 0.5)
  (`self.Reset movimiento`))

(event `self.ReceiveBeginPlay`
  (goto _label))

(fn `UserConstructionScript`)