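; BP_PlataformaMovil2 is a moving platform that travels vertically up and down in an endless loop from BeginPlay.
; Latent MoveComponentTo nodes move the root component 800 units up and then back down over four seconds each way, with a short pause after each move.
; The custom event ResetMovimientp calls itself at the end to repeat the cycle, taking each target from the current actor location.
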(event `Reset Movimientp`
  (`KismetSystemLibrary.MoveComponentTo` (`self.DefaultSceneRoot`) (+ (`self.K2_GetActorLocation`) (0.0 0.0 800.0)) (struct) false false 4.0 :!label _label)
  (`KismetSystemLibrary.Delay` 0.5)
  (`KismetSystemLibrary.MoveComponentTo` (`self.DefaultSceneRoot`) (+ (`self.K2_GetActorLocation`) (0.0 0.0 -800.0)) (struct) false false 4.0)
  (`KismetSystemLibrary.Delay` 0.5)
  (`self.Reset Movimientp`))

(event `self.ReceiveBeginPlay`
  (goto _label))

(fn `UserConstructionScript`)